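; Base interactable Blueprint for hold-to-interact objects, with an empty Action event as the hook for the completed interaction.
; Interact creates a W_Interact_Loadbar and starts a looping timer that builds hold time, feeding the widget until the limit triggers Action and removes it.
; Released removes the bar and starts a second timer that drains unfinished progress gradually instead of resetting it.
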(event `self.Interact`
  (bind _returnvalue (`|CreateWidget` "/Game/Content/UI/Interactables/W_Interact_Loadbar.W_Interact_Loadbar_C" (`GameplayStatics.GetPlayerController` 0) (`self.ButtonPushLimit`)))
  (bind _output_get (set `self.W_Interact_Loadbar_Ref` _returnvalue))
  (`UserWidget.AddToViewport` _output_get 0)
  (`self.Held`))

(event `self.Action`)

(event `Held`
  (`KismetSystemLibrary.K2_ClearAndInvalidateTimerHandle` (`self.ButtonReleaseTimer`))
  (bind _returnvalue (`KismetSystemLibrary.K2_SetTimer` null "HandleButtonHeldTImer" 0.01 true))
  (set `self.ButtonHeldTimer` _returnvalue))

(event `self.Released`
  (`KismetSystemLibrary.K2_ClearAndInvalidateTimerHandle` (`self.ButtonHeldTimer`))
  (bind _returnvalue (`KismetSystemLibrary.K2_SetTimer` null "HandleButtonReleaseTimer" 0.01 true))
  (set `self.ButtonReleaseTimer` _returnvalue)
  (`self.RemoveLoadbar`))

(fn `HandleButtonHeldTImer`
  (if (> (`self.ButtonPushTime`) (`self.ButtonPushLimit`))
    (`self.Action`)
    (`KismetSystemLibrary.K2_ClearAndInvalidateTimerHandle` (`self.ButtonHeldTimer`))
    (`self.RemoveLoadbar`)
    (else
      (set `self.ButtonPushTime` (+ (`self.ButtonPushTime`) 0.01))
      (`self.UpdateWidget`))))

(fn `HandleButtonReleaseTimer`
  (bind _buttonpushtime (`self.ButtonPushTime`))
  (if (and (> (`self.ButtonPushLimit`) _buttonpushtime) (> _buttonpushtime 0.0))
    (set `self.ButtonPushTime` (- (`self.ButtonPushTime`) 0.01))
    (`self.UpdateWidget`)
    (else
      (`KismetSystemLibrary.K2_ClearAndInvalidateTimerHandle` (`self.ButtonHeldTimer`)))))

(fn `RemoveLoadbar`
  (bind _w_interact_loadbar_ref (`self.W_Interact_Loadbar_Ref`))
  (`/Engine/EditorBlueprintResources/StandardMacros.IsValid` _w_interact_loadbar_ref
    (:`Is Valid`
      (`Widget.RemoveFromParent` _w_interact_loadbar_ref))
    (:`Is Not Valid`
      _))
  (set `self.W_Interact_Loadbar_Ref` null))

(fn `UpdateWidget`
  (bind _w_interact_loadbar_ref (`self.W_Interact_Loadbar_Ref`))
  (`/Engine/EditorBlueprintResources/StandardMacros.IsValid` _w_interact_loadbar_ref
    (:`Is Valid`
      (set `/Game/Content/UI/Interactables/W_Interact_Loadbar.ButtonPushHeld` (`self.ButtonPushTime`) _w_interact_loadbar_ref))))

(fn `UserConstructionScript`)